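; BP_ArcadeMachine is an arcade cabinet actor that plays Asteroids videos on its screen and acts as a coin-operated door trigger.
; On begin play, ArcadeMedia loops a loading video.
; A BP_ArcadeCoin overlapping CoinSlot spawns confetti, is destroyed, and after a delay starts the gameplay video once.
; When that video ends, the screen swaps to an end-screen material and OpenDoorWithID opens door "2".
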(event `self.CoinSlot.OnComponentBeginOverlap`
  (params (OverlappedComponent :type "PrimitiveComponent Object Reference") (OtherActor :type "Actor Object Reference") (OtherComp :type "PrimitiveComponent Object Reference") (OtherBodyIndex :type Integer) (bFromSweep :type Boolean) (SweepResult :type "HitResult Structure (by ref)"))
  (bind _arcademedia (`self.ArcadeMedia`))
  (bind _asbp_arcade_coin (cast `/Game/_Imported/ArcadeCoin/BP_ArcadeCoin` OtherActor))
  (`NiagaraFunctionLibrary.SpawnSystemAtLocation` "/Game/_Imported/M_ArcadeMachine/Confetti.Confetti" (`self.K2_GetActorLocation` _asbp_arcade_coin) (struct) (0.01 0.01 0.01))
  (`self.K2_DestroyActor` _asbp_arcade_coin)
  (`KismetSystemLibrary.Delay` 3.5)
  (`MediaPlayer.OpenSource` _arcademedia "/Game/_Imported/M_ArcadeMachine/Media/AsteroidsGameplay.AsteroidsGameplay")
  (`MediaPlayer.SetLooping` _arcademedia false)
  (`MediaPlayer.Play` _arcademedia)
  (add `MediaPlayer.OnEndReached` _arcademedia (delegate `EndReached`)))

(event `self.ReceiveBeginPlay`
  (bind _arcademedia (`self.ArcadeMedia`))
  (`MediaPlayer.OpenSource` _arcademedia "/Game/_Imported/M_ArcadeMachine/Media/AsteroidsGameLoading.AsteroidsGameLoading")
  (`MediaPlayer.SetLooping` _arcademedia true)
  (`MediaPlayer.Play` _arcademedia))

(event `EndReached`
  (`PrimitiveComponent.SetMaterial` (`self.Screen`) 0 "/Game/_Imported/M_ArcadeMachine/Materials/End_Screen.End_Screen")
  (`/Game/Blueprints/BFL_GameFunctions.OpenDoorWithID` "2"))

(fn `UserConstructionScript`)